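; Timed effect anim notify state that drives an elemental Niagara trail during an animation.
; Each notify tick gets the spawned effect and writes the mesh's Start and End socket locations into its StartTrail and EndTrail vector parameters, so the trail follows those sockets.
; If no valid effect exists, it prints a "Trail Not Valid" message.
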(fn ReceivedNotifyTick
  (params (MeshComp :type Skeletal%20Mesh%20Component%20Object%20Reference) (Animation :type Anim%20Sequence%20Base%20Object%20Reference) (FrameDeltaTime :type Float%20%28single-precision%29))
  (bind _returnvalue (Class|AnimNotifyStateTimedNiagaraEffect|GetSpawnedEffect MeshComp))
  (Utilities|IsValid _returnvalue
    (:Is%20Valid
      (Effects|Components|ParticleSystem|SetVectorParameter _returnvalue "StartTrail" (Transformation|GetSocketLocation MeshComp (Variables|Default|GetStart)))
      (Effects|Components|ParticleSystem|SetVectorParameter _returnvalue "EndTrail" (Transformation|GetSocketLocation MeshComp (Variables|Default|GetEnd)))
      (return false))
    (:Is%20Not%20Valid
      (Development|PrintString 0 "Trail Not Valid")
      (return false))))