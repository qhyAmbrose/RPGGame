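; ZombieAIBP is a zombie AI Blueprint with an attribute component whose health-change event is bound but currently does nothing.
; Disconnected, never-executed logic would show a damage popup and play a roar for major hits, both using NewValue rather than Delta as the amount.
; Its death branch would attach a sound, with no asset set, to the mesh so it follows the ragdoll.
; The construction script is empty.
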(event OnHealthChanged(AttributeComp)
  (params (InstigatorActor :type Actor%20Object%20Reference) (OwningComp :type My%20Attribute%20Component%20Object%20Reference) (NewValue :type Float%20%28single-precision%29) (Delta :type Float%20%28single-precision%29)))

(fn ConstructionScript)